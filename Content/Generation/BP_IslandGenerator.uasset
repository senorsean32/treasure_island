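; Server-authoritative generator that populates the level with a random number of islands and hides treasure on some of them at BeginPlay.
; It clears existing BP_Island_Base actors, then spawns new ones at random XY points within the first BP_Water actor's bounds, at zero height.
; Treasure placement flags random islands, reveals their meshes and updates the game mode's TreasuresRemaining, recursing until it reaches TreasureCount.
; A helper returns the islands holding treasure.
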(event `self.ReceiveBeginPlay`
  (`|ExecutionSequence`
    (:`then_0`
      (`self.GetReferences`))
    (:`then_1`
      (`/Engine/EditorBlueprintResources/ActorMacros.Switch Has Authority`
        (:`Authority`
          (`self.GenerateIslands`))))))

(event `GenerateIslands`
  (`/Engine/EditorBlueprintResources/ActorMacros.Switch Has Authority`
    (:`Authority`
      (`|ExecutionSequence`
        (:`then_0`
          (`self.Clear Islands`))
        (:`then_1`
          (bind _outactors (`GameplayStatics.GetAllActorsOfClass` "/Game/WorldElements/BP_Water.BP_Water_C"))
          (set `self.WaterRef` (`|GetArrayItem` _outactors)))
        (:`then_2`
          (`self.CreateIslands` (`self.GetRandomIslandCount`) (`self.WaterRef`))
          (`self.Hide Treasure on Islands`))))))

(event `Hide Treasure on Islands`
  (bind _gamemoderef (`self.GameModeRef`))
  (bind _gamemoderef_2 (`self.GameModeRef`))
  (bind _islandslist (`self.IslandsList`))
  (bind _output (`|GetArrayItem` _islandslist (`KismetMathLibrary.RandomIntegerInRange` 0 (`KismetArrayLibrary.Array_Length` _islandslist))))
  (bind _treasuremesh (`/Game/WorldElements/BP_Island_Base.TreasureMesh` _output))
  ;[1 1 1] Randomly set an Island to have treasure
  (`/Engine/EditorBlueprintResources/ActorMacros.Switch Has Authority`
    (:`Authority`
      (if (< (`/Game/GameManagers/GameMode_Default.TreasuresRemaining` _gamemoderef_2) (`/Game/GameManagers/GameMode_Default.TreasureCount` _gamemoderef_2))
        (for _ (range 1 (+ (`/Game/GameManagers/GameMode_Default.TreasureCount` (`self.GameModeRef`)) 1))
          (if (not (`/Game/WorldElements/BP_Island_Base.HasTreasure` _output))
            (set `/Game/WorldElements/BP_Island_Base.HasTreasure` true _output)
            (`/Engine/EditorBlueprintResources/StandardMacros.IsValid` _treasuremesh
              (:`Is Valid`
                (`SceneComponent.SetVisibility` _treasuremesh true false)
                (bind _result (`/Engine/EditorBlueprintResources/StandardMacros.IncrementInt` (`/Game/GameManagers/GameMode_Default.TreasuresRemaining` (`self.GameModeRef`)))
                  (:`  `
                    (set `/Game/GameManagers/GameMode_Default.TreasuresRemaining` _result (`self.GameModeRef`))))))))
        ;;[1 1 1] If all treasures have not been placed do it again
        (if (< (`/Game/GameManagers/GameMode_Default.TreasuresRemaining` _gamemoderef) (`/Game/GameManagers/GameMode_Default.TreasureCount` _gamemoderef))
          (`self.Hide Treasure on Islands`))))))

(event `Clear Islands`
  ;[1 1 1] Clear the islands (called in editor)
  (`/Engine/EditorBlueprintResources/ActorMacros.Switch Has Authority`
    (:`Authority`
      (set `/Game/GameManagers/GameMode_Default.TreasuresRemaining` 0 (`self.GameModeRef`))
      (bind _outactors (`GameplayStatics.GetAllActorsOfClass` "/Game/WorldElements/BP_Island_Base.BP_Island_Base_C"))
      (for _array_element _outactors
        (`KismetArrayLibrary.Array_RemoveItem` (`self.IslandsList`) _array_element)
        (`self.K2_DestroyActor` _array_element)))))

(fn `CreateIslands`
  (params (IslandsCount :type Integer) (`Water Reference` :type "Actor Object Reference"))
  (bind (_origin _boxextent) (`self.GetActorBounds` `Water Reference` false))
  (bind (_returnvalue_x _returnvalue_y) (`KismetMathLibrary.BreakVector` (`KismetMathLibrary.RandomPointInBoundingBox` _origin _boxextent)))
  (for _ (range 1 (+ IslandsCount 1))
    (bind _returnvalue (`|SpawnActorFromClass` "/Game/WorldElements/BP_Island_Base.BP_Island_Base_C" (`KismetMathLibrary.MakeTransform` (`KismetMathLibrary.MakeVector` _returnvalue_x _returnvalue_y)) "Undefined" "OverrideRootScale" null null))
    (`/Engine/EditorBlueprintResources/StandardMacros.IsValid` _returnvalue
      (:`Is Valid`
        (`KismetArrayLibrary.Array_Add` (`self.IslandsList`) _returnvalue)))))

(fn `Get Islands with Treasure`
  (returns (`Islands with Treasure` :type "Array of /Game/WorldElements/BP_Island_Base Object Reference"))
  (locals (_islandsWithTreasure :type "Array of /Game/WorldElements/BP_Island_Base Object Reference"))
  (for _array_element (`self.IslandsList`)
    (if (== (`/Game/WorldElements/BP_Island_Base.HasTreasure` _array_element) true)
      (`KismetArrayLibrary.Array_AddUnique` (`local._islandsWithTreasure`) _array_element)))
  (return (`local._islandsWithTreasure`)))

(fn `GetRandomIslandCount`
  (returns (ReturnValue :type Integer))
  (return (`KismetMathLibrary.RandomIntegerInRange` (`self.IslandsMin`) (`self.IslandsMax`))))

(fn `GetReferences`
  (bind _asgame_mode_default (cast `/Game/GameManagers/GameMode_Default` (`GameplayStatics.GetGameMode`)))
  (set `self.GameModeRef` _asgame_mode_default))

(fn `UserConstructionScript`)