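; Base player-controlled ship that sails with smoothed throttle, server-routed steering and an orbit/zoom camera.
; Tick adds sine-wave bobbing and rocking, with roll damped by speed, and toggles wake particles by velocity.
; Interact, on authority, sphere-searches for the closest island, spawns a BP_Player toward it, possesses it and stops the ship.
; A delayed BeginPlay hack picks a random GameMode hull color, sent through server and multicast events, with an OnRep updating materials.
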(event `self.ReceiveBeginPlay`
  ;[0 1 0.01226] Begin Play
  (`KismetSystemLibrary.Delay` 0.1)
  (`self.SetShipColorHACK!!!`))

(event `self.ReceiveTick`
  (params (DeltaSeconds :type "Float (single-precision)"))
  ;[1 0 0] Tick
  (`self.ShipMeshMovement` 2.0 2.0 2.0)
  (`self.TryPlayWakeFX`))

(event `InputAxis|Input_FwdBwd`
  (params (AxisValue :type "Float (single-precision)"))
  (bind _returnvalue (`KismetMathLibrary.FInterpTo` (`self.InputFwd_LastFrame`) (* (* AxisValue (`self.MoveSpeed`)) (`GameplayStatics.GetWorldDeltaSeconds`)) (`GameplayStatics.GetWorldDeltaSeconds`) 5.0))
  ;[1 1 1] Movement and Camera Input Hanlding
  (`self.AddMovementInput` (`self.GetActorForwardVector`) _returnvalue)
  (set `self.InputFwd_LastFrame` _returnvalue))

(event `SteerShip_SVR`
  (params (TurnDelta :type "Float (double-precision)"))
  ;[1 1 1] Movement and Camera Input Hanlding
  (`self.K2_AddActorWorldRotation` (`KismetMathLibrary.MakeRotator` 0.0 0.0 TurnDelta)))

(event `InputAxis|Input_LeftRight`
  (params (AxisValue :type "Float (single-precision)"))
  ;[1 1 1] Movement and Camera Input Hanlding
  (`self.SteerShip_SVR` (* (* AxisValue (`self.TurnRate`)) (`GameplayStatics.GetWorldDeltaSeconds`))))

(event `InputAxis|MouseX`
  (params (AxisValue :type "Float (single-precision)"))
  ;[1 1 1] Movement and Camera Input Hanlding
  (`self.AddControllerYawInput` AxisValue))

(event `InputAxis|MouseY`
  (params (AxisValue :type "Float (single-precision)"))
  ;[1 1 1] Movement and Camera Input Hanlding
  (`self.AddControllerPitchInput` (* AxisValue -1.0)))

(event `self.ReceivePossessed`
  (params (NewController :type "Controller Object Reference"))
  ;[1 1 1] Get ref to Player Controller
  (bind _asplayer_controller_default (cast `/Game/GameManagers/PlayerController_Default` NewController))
  (set `self.PlayerControllerRef` _asplayer_controller_default)
  ;[1 1 1] Allows Player Controller to know which ship belongs to the player
  (set `/Game/GameManagers/PlayerController_Default.PlayerInfo` (make `/Game/StructsAndEnums/S_PlayerInfo` "Player1" self) (`self.PlayerControllerRef`)))

(event `InputAxis|MouseWheel`
  (params (AxisValue :type "Float (single-precision)"))
  ;[1 1 1] Movement and Camera Input Hanlding
  (`self.CameraZoom` AxisValue))

(event `SetShipColor_SVR`
  (params (ShipColor :type "LinearColor Structure"))
  ;[1 1 1] Set Ship Color with Replication
  (bind _output_get (set `self.ShipColor` ShipColor))
  (`self.SetShipColor_MULTI` _output_get))

(event `InputAction|Interact`
  (params (Key :type "Key Structure"))
  ;[1 1 1] Input to for Try Board Island
  (:`Pressed`
    (`self.TryBoardIsland`)))

(event `SetShipColor_MULTI`
  (params (ShipColor :type "LinearColor Structure"))
  ;[1 1 1] Set Ship Color with Replication
  (set `self.ShipColor` ShipColor))

(event `TryBoardIsland`
  ;[1 1 1] Try to board an island event called on server
  (`/Engine/EditorBlueprintResources/ActorMacros.Switch Has Authority`
    (:`Authority`
      (bind (_hasfound _islandslist) (`self.SearchForIsland` (`self.IslandCastRadius`)))
      (if _hasfound
        (bind _bestislandreturn (`self.SelectBestIsland` _islandslist))
        (bind (_spawnloc _spawnrot) (`self.FindPlayerSpawnOnIsland` _bestislandreturn (`self.DistanceFromShipSpawn`)))
        (bind _returnvalue (`|SpawnActorFromClass` "/Game/Pawns/BP_Player.BP_Player_C" (`KismetMathLibrary.MakeTransform` _spawnloc _spawnrot) "AlwaysSpawn" "OverrideRootScale" null null))
        (`Controller.Possess` (`self.PlayerControllerRef`) _returnvalue)
        ;[1 1 1] Stop ship movement on server and all clients
        (`/Engine/EditorBlueprintResources/ActorMacros.Switch Has Authority`
          (:`Authority`
            _)
          (:`Remote`
            _))
        (`MovementComponent.StopMovementImmediately` (`self.CharacterMovement`))))))

(fn `CameraZoom`
  (params (AxisValue :type "Float (double-precision)"))
  (locals (ZoomSpeed :type "Float (double-precision)" :default 200.0) (ArmLength_LastFrame :type "Float (double-precision)"))
  (bind _springarm (`self.SpringArm`))
  (bind _returnvalue (`KismetMathLibrary.FClamp` (+ (`SpringArmComponent.TargetArmLength` _springarm) (* (* AxisValue -1.0) (`local.ZoomSpeed`))) 300.0 6000.0))
  (set `SpringArmComponent.TargetArmLength` _returnvalue _springarm)
  (set `local.ArmLength_LastFrame` _returnvalue))

(fn `FindPlayerSpawnOnIsland`
  (params (IslandRef :type "/Game/WorldElements/BP_Island_Base Object Reference") (DistanceFromShip :type "Float (double-precision)"))
  (returns (SpawnLoc :type "Vector Structure") (SpawnRot :type "Rotator Structure"))
  (locals (_distFromShipToSpawn :type "Float (double-precision)") (_islandRef :type "/Game/WorldElements/BP_Island_Base Object Reference") (_shipLocation :type "Vector Structure"))
  (bind (_returnvalue_roll _returnvalue_pitch _returnvalue_yaw) (`KismetMathLibrary.BreakRotator` (`SceneComponent.K2_GetComponentRotation` (`self.Camera`))))
  ;[1 1 1] Local var refs
  (set `local._islandRef` IslandRef)
  (set `local._distFromShipToSpawn` DistanceFromShip)
  (set `local._shipLocation` (`self.K2_GetActorLocation`))
  (return (+ (* (`KismetMathLibrary.GetForwardVector` (`KismetMathLibrary.FindLookAtRotation` (`local._shipLocation`) (`self.K2_GetActorLocation` (`local._islandRef`)))) (`local._distFromShipToSpawn`)) (`local._shipLocation`)) (`KismetMathLibrary.MakeRotator` 0.0 0.0 _returnvalue_yaw)))

(fn `OnRep_ShipColor`
  (`MeshComponent.SetVectorParameterValueOnMaterials` (`self.ShipBase`) "BaseColor" (`KismetMathLibrary.Conv_LinearColorToVector` (`self.ShipColor`))))

(fn `SearchForIsland`
  (params (SphereRadius :type "Float (double-precision)"))
  (returns (HasFound :type Boolean) (IslandsList :type "Array of /Game/WorldElements/BP_Island_Base Object Reference"))
  (locals (IslandList :type "Array of /Game/WorldElements/BP_Island_Base Object Reference") (hasFoundIsland :type Boolean) (SphereRad :type "Float (double-precision)"))
  ;[1 1 1] Initial Variable Settings
  (set `local.SphereRad` SphereRadius)
  (set `local.hasFoundIsland` false)
  (`KismetArrayLibrary.Array_Clear` (`local.IslandList`))
  ;[1 1 1] Sphere Cast looking for Island Actors
  (bind _outactors (`KismetSystemLibrary.SphereOverlapActors` (`self.K2_GetActorLocation`) (`local.SphereRad`) (`|MakeArray` "ObjectTypeQuery1" "ObjectTypeQuery2" :!type "EObjectTypeQuery Enum") "/Game/WorldElements/BP_Island_Base.BP_Island_Base_C"))
  ;[1 1 1] Loop thru actors and add any Islands to the List
  (for _array_element _outactors
    (bind _asbp_island_base (cast `/Game/WorldElements/BP_Island_Base` _array_element))
    (`KismetArrayLibrary.Array_Add` (`local.IslandList`) _asbp_island_base)
    (set `local.hasFoundIsland` true))
  ;[1 1 1] If any island was found return True and List of islands. Else return False and empty list
  (if (`local.hasFoundIsland`)
    (return true (`local.IslandList`))
    (else
      (return false))))

(fn `SelectBestIsland`
  (params (IslandList :type "Array of /Game/WorldElements/BP_Island_Base Object Reference"))
  (returns (BestIslandReturn :type "/Game/WorldElements/BP_Island_Base Object Reference"))
  (locals (_islandList :type "Array of /Game/WorldElements/BP_Island_Base Object Reference") (BestIsland :type "/Game/WorldElements/BP_Island_Base Object Reference") (ClosestIslandDistance :type "Float (double-precision)" :default 10000000.0))
  ;[1 1 1] Store a local var ref
  (set `local._islandList` IslandList)
  ;[1 1 1] Check that the Island list isnt empty, if so notify dev
  (if (<= (`KismetArrayLibrary.Array_Length` (`local._islandList`)) 0)
    (`KismetSystemLibrary.PrintString` "Cannot select the best island of an empty island list")
    (return null)
    (else
      ;[1 1 1] Found closest island
      (for _array_element (`local._islandList`)
        (bind _returnvalue (`self.GetHorizontalDistanceTo` _array_element))
        (if (< _returnvalue (`local.ClosestIslandDistance`))
          (set `local.ClosestIslandDistance` _returnvalue)
          (set `local.BestIsland` _array_element)))
      ;[1 1 1 1 15] Return best Island
      (return (`local.BestIsland`)))))

(fn `SetShipColorHACK!!!`
  (bind _asgame_mode_default (cast `/Game/GameManagers/GameMode_Default` (`GameplayStatics.GetGameMode`)))
  (bind _shipcolor (`/Game/GameManagers/GameMode_Default.ShipColor` _asgame_mode_default))
  (bind _output (`|GetArrayItem` _shipcolor (`KismetMathLibrary.RandomIntegerInRange` 0 (`KismetArrayLibrary.Array_Length` _shipcolor))))
  (`KismetArrayLibrary.Array_RemoveItem` _shipcolor _output)
  (`self.SetShipColor_SVR` _output))

(fn `ShipMeshMovement`
  (params (RollAmt :type "Float (double-precision)") (PitchAmt :type "Float (double-precision)") (TimeScale :type "Float (double-precision)"))
  (bind (_returnvalue_roll _returnvalue_pitch _returnvalue_yaw) (`KismetMathLibrary.BreakRotator` (`SceneComponent.K2_GetComponentRotation` (`self.ShipBase`))))
  (bind _returnvalue (`KismetMathLibrary.Sin` (* (`GameplayStatics.GetTimeSeconds`) TimeScale)))
  (`|ExecutionSequence`
    (:`then_0`
      ;[1 1 1] Water Translation Effect
      (`SceneComponent.K2_AddWorldOffset` (`self.ShipBase`) (`KismetMathLibrary.MakeVector` 0.0 0.0 (* (`KismetMathLibrary.Sin` (* (`GameplayStatics.GetTimeSeconds`) TimeScale)) 0.075)) false false))
    (:`then_1`
      ;[1 1 1] Water Rotation Effects
      (`SceneComponent.K2_SetWorldRotation` (`self.ShipBase`) (`KismetMathLibrary.MakeRotator` (+ 180.0 (* (* _returnvalue RollAmt) (`KismetMathLibrary.MapRangeClamped` (`KismetMathLibrary.VSize` (`self.GetVelocity`)) 0.0 600.0 1.0 0.2))) (+ 0.0 (* _returnvalue PitchAmt)) _returnvalue_yaw) false false))))

(fn `SteerShip`
  (params (TurnDeltaIn :type "Float (double-precision)"))
  (returns (TurnDeltaOut :type "Float (double-precision)"))
  (`self.K2_AddActorWorldRotation` (`KismetMathLibrary.MakeRotator` 0.0 0.0 TurnDeltaIn))
  (return TurnDeltaIn))

(fn `TryPlayWakeFX`
  (bind (_returnvalue_x _returnvalue_y) (`KismetMathLibrary.BreakVector` (`self.GetVelocity`)))
  (if (> (`KismetMathLibrary.VSize` (`KismetMathLibrary.MakeVector` _returnvalue_x _returnvalue_y)) 30.0)
    (`ActorComponent.Activate` (`self.WakeParticle`) false)
    (else
      (`ActorComponent.Deactivate` (`self.WakeParticle`)))))

(fn `UserConstructionScript`)