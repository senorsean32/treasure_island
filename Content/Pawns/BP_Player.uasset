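; BP_Player is the player pawn, with axis-driven movement, mouse look and an early stub for boarding ships.
; On BeginPlay it binds an event to PlayerController_Default's interact hook.
; TryBoardShip runs only with authority and so far just prints the name of the player's owned ship.
; SearchForShip finds a nearby BP_Ship_Base by sphere overlap, but its only call is in unconnected logic.
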(event `InputAxis|Input_FwdBwd`
  (params (AxisValue :type "Float (single-precision)"))
  ;[1 1 1] Input Handling
  (`self.AddMovementInput` (`self.GetActorForwardVector`) (* (* AxisValue (`self.MoveSpeed`)) (`GameplayStatics.GetWorldDeltaSeconds`))))

(event `self.ReceiveBeginPlay`
  ;[1 1 1] Quick n Dirty binding to PC input
  (bind _asplayer_controller_default (cast `/Game/GameManagers/PlayerController_Default` (`self.GetController`)))
  (add `/Game/GameManagers/PlayerController_Default.TryInteract` _asplayer_controller_default (`|CreateDelegate` :!event `TryBoardShip`)))

(event `InputAxis|Input_LeftRight`
  (params (AxisValue :type "Float (single-precision)"))
  ;[1 1 1] Input Handling
  (`self.AddMovementInput` (`self.GetActorRightVector`) (* (* AxisValue (`self.MoveSpeed`)) (`GameplayStatics.GetWorldDeltaSeconds`))))

(event `InputAxis|MouseX`
  (params (AxisValue :type "Float (single-precision)"))
  ;[1 1 1] Input Handling
  (`self.AddControllerYawInput` AxisValue))

(event `TryBoardShip`
  (`/Engine/EditorBlueprintResources/ActorMacros.Switch Has Authority`
    (:`Authority`
      (bind _asplayer_controller_default (cast `/Game/GameManagers/PlayerController_Default` (`self.GetController`)))
      (bind (_playerinfo_playername _playerinfo_ownedship) (break `/Game/StructsAndEnums/S_PlayerInfo` (`/Game/GameManagers/PlayerController_Default.PlayerInfo` _asplayer_controller_default)))
      (`KismetSystemLibrary.PrintString` (`KismetStringLibrary.Concat_StrStr` "Trying to board " (`KismetSystemLibrary.GetDisplayName` _playerinfo_ownedship))))))

(event `InputAxis|MouseY`
  (params (AxisValue :type "Float (single-precision)"))
  ;[1 1 1] Input Handling
  (`self.AddControllerPitchInput` (* AxisValue -1.0)))

(event `InputAction|Interact`
  (params (Key :type "Key Structure"))
  ;[1 1 1] Input Handling
)

(fn `SearchForShip`
  (returns (`Found Ship Ref` :type "/Game/Pawns/BP_Ship_Base Object Reference"))
  (locals (IslandCastRadius :type "Float (double-precision)" :default 500.0))
  (bind _outactors (`KismetSystemLibrary.SphereOverlapActors` (`self.K2_GetActorLocation`) 300.0 (`|MakeArray` "ObjectTypeQuery3" :!type "EObjectTypeQuery Enum") "/Game/Pawns/BP_Ship_Base.BP_Ship_Base_C"))
  (bind _asbp_ship_base (cast `/Game/Pawns/BP_Ship_Base` (`|GetArrayItem` _outactors))
    (:`then`
      (return _asbp_ship_base))
    (:`CastFailed`
      (return null))))

(fn `UserConstructionScript`)