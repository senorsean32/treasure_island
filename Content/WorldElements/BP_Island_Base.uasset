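; Base island actor that randomizes its footprint and can reveal a treasure.
; When ExecConstrutionScript is set, the construction script scales the mesh's X and Y by one random factor within the configured range, keeping Z fixed.
; It then sizes the Sphere component from the actor's horizontal bounds plus CollisionBuffer.
; The ShowTreasure event sets HasTreasure and makes TreasureMesh and its children visible.
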(event `ShowTreasure`
  (set `self.HasTreasure` true)
  (`SceneComponent.SetVisibility` (`self.TreasureMesh`) true true))

(fn `UserConstructionScript`
  (locals (CollisionBuffer :type "Float (double-precision)" :default 300.0))
  (bind (_returnvalue_x _returnvalue_y _returnvalue_z) (`KismetMathLibrary.BreakVector` (`KismetMathLibrary.MakeVector` 20.0 20.0 0.25)))
  (bind (_origin _boxextent) (`self.GetActorBounds` false))
  (if (`self.ExecConstrutionScript`)
    (set `self.IslandScaleFactor` (`KismetMathLibrary.RandomFloatInRange` (`self.IslandScaleFactor_Min`) (`self.IslandScaleFactor_Max`)))
    (set `self.IslandScale` (`KismetMathLibrary.MakeVector` (* _returnvalue_x (`self.IslandScaleFactor`)) (* _returnvalue_y (`self.IslandScaleFactor`)) _returnvalue_z))
    (`SceneComponent.SetRelativeScale3D` (`self.StaticMesh`) (`self.IslandScale`))
    (`SphereComponent.SetSphereRadius` (`self.Sphere`) (+ (* (+ (.x _boxextent) (.y _boxextent)) 2.0) (`local.CollisionBuffer`)) true)))